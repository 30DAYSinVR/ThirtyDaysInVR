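; WaveVR player character for PlanetWalker, offering gaze pointing, object spawning, run-in-place locomotion and a jetpack.
; Each Tick traces the view ray to position and scale the reticle and spawn actors at hits, hiding it when the system captures input.
; Toggleable run-in-place turns smoothed vertical head motion into forward movement.
; The jetpack adds lift plus HMD-relative touchpad thrust, with velocity clamped; planet surface alignment is unwired.
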(event `self.ReceiveBeginPlay`
  (`HeadMountedDisplayFunctionLibrary.SetTrackingOrigin` "Eye")
  (`SceneComponent.K2_SetRelativeLocation` (`self.VRCameraRoot`) (`self.CameraHeight`) false false))

(event `self.ReceiveTick`
  (params (DeltaSeconds :type "Float (single-precision)"))
  (bind _headrelativevel (`self.HeadRelativeVel`))
  (bind _ripmotionsmoothingsteps (`self.RIPMotionSmoothingSteps`))
  (bind _jetpackverticalforce (`self.JetpackVerticalForce`))
  (bind _rpscreendistance (`self.rpScreenDistance`))
  (bind _reticlepointer (`self.ReticlePointer`))
  (bind _returnvalue (`SceneComponent.GetComponentVelocity` (`self.CapsuleComponent`)))
  (bind _z (.z (`self.HeadRelativeVel`)))
  (bind (_outlocation _outrotation) (`self.GetActorEyesViewPoint` (`GameplayStatics.GetPlayerCameraManager` 0)))
  (bind _returnvalue_2 (`KismetMathLibrary.FClamp` (`self.traceDist`) (`self.rpMinDist`) _rpscreendistance))
  (bind _relativelocation (`SceneComponent.RelativeLocation` (`self.VRCamera`)))
  (`|ExecutionSequence`
    (:`then_0`
      (bind _returnvalue_3 (`WaveVRBlueprintFunctionLibrary.IsInputFocusCapturedBySystem`))
      ;[1 1 1] Enable/Disable Menu interaction
      (`ActorComponent.SetActive` (`self.WidgetInteraction_Menu`) (not _returnvalue_3) false)
      ;[1 1 1] RETICLE POINTER SYSTEM
      ;;[1 1 1] Enable/Disable Reticle Point
      (`self.SetActorHiddenInGame` (`ActorComponent.GetOwner` (`self.ReticlePointer`)) _returnvalue_3)
      (bind (_outhit _returnvalue_4) (`KismetSystemLibrary.LineTraceSingle` _outlocation (+ _outlocation (* (`KismetMathLibrary.Conv_RotatorToVector` _outrotation) (`self.rpScreenDistance`))) "TraceTypeQuery2"))
      (if _returnvalue_4
        (bind (_bblockinghit _binitialoverlap _time _location _impactpoint) (`GameplayStatics.BreakHitResult` _outhit))
        (bind _output_get (set `self.traceDist` (`KismetMathLibrary.VSize` (- _impactpoint _outlocation))))
        (set `self.savedTraceDist` _output_get)
        (else
          (set `self.traceDist` (`self.savedTraceDist`))))
      (`SceneComponent.K2_SetRelativeLocation` _reticlepointer (* (`KismetMathLibrary.Conv_DoubleToVector` (- _returnvalue_2 (`self.rpConstSurfaceOffset`))) (1.0 0.0 0.0)) false false)
      (`SceneComponent.SetRelativeScale3D` _reticlepointer (`KismetMathLibrary.Conv_DoubleToVector` (* (`KismetMathLibrary.FMin` (* _returnvalue_2 (/ (`self.rpScaleOffset`) _rpscreendistance)) 1.0) (`self.rpScaleSize`))))
      ;[1 1 1] Spawn Object at eye ray position
      (bind _returnvalue_5 (`WaveVRController.IsRightControllerButtonPressedDown` "DPad_Up"))
      (if _returnvalue_5
        (`|SpawnActorFromClass` (`self.ActorToSpawn`) (`KismetMathLibrary.MakeTransform` (+ _impactpoint (0.0 0.0 200.0))) "AdjustIfPossibleButAlwaysSpawn" "OverrideRootScale" null null)))
    (:`then_1`
      ;[1 1 1] On/Off Run In Place
      (bind _returnvalue_6 (`WaveVRController.IsRightControllerButtonPressedDown` "Menu"))
      (if _returnvalue_6
        (set `self.isRunInPlaceActive` (not (`self.isRunInPlaceActive`)))))
    (:`then_2`
      ;[1 1 1] RUN IN PLACE SYSTEM
      (if (`self.isRunInPlaceActive`)
        ;;[1 1 1] Rolling Average in blueprint
        (set `self.HeadRelativeVel` (+ (- _headrelativevel (/ _headrelativevel _ripmotionsmoothingsteps)) (/ (`KismetMathLibrary.MakeVector` (`KismetMathLibrary.Abs` (.x (- _relativelocation (`self.LastHDMPosition`)))) (`KismetMathLibrary.Abs` (.y (- _relativelocation (`self.LastHDMPosition`)))) (`KismetMathLibrary.Abs` (.z (- _relativelocation (`self.LastHDMPosition`))))) _ripmotionsmoothingsteps)))
        (set `self.LastHDMPosition` _relativelocation)
        ;;[1 1 1] If moving more than threshold
        (if (>= _z (`self.MinimumRIPVelocity`))
          ;;[1 1 1] Apply Movement Input
          (`self.AddMovementInput` (* (`SceneComponent.GetForwardVector` (`self.VRCamera`)) (1.0 1.0 0.0)) (`KismetMathLibrary.FClamp` (* (`self.RunInPlaceScaler`) _z))))
        (else
          ;;[1 1 1] Reset movement vectors
          (`|ExecutionSequence`
            (:`then_0`
              (set `self.LastHDMPosition` (0.0 0.0 0.0)))
            (:`then_1`
              (set `self.HeadRelativeVel` (0.0 0.0 0.0)))))))
    (:`then_3`
      ;[1 1 1] Jetpack system with dpad direction
      (bind _returnvalue_7 (`WaveVRController.IsRightControllerButtonPressed` "Bumper"))
      (if _returnvalue_7
        (bind (_outposition _outorientation) (`WaveVRBlueprintFunctionLibrary.GetDevicePose` "DeviceType_HMD"))
        (bind _returnvalue_8 (`WaveVRController.GetRightControllerAxis` "Touchpad"))
        (bind _returnvalue_9 (`WaveVRController.IsRightControllerButtonTouched` "Touchpad"))
        (if _returnvalue_9
          (bind (_returnvalue_x _returnvalue_y) (`KismetMathLibrary.BreakVector` (* (`KismetMathLibrary.GreaterGreater_VectorRotator` (`KismetMathLibrary.MakeVector` (`KismetMathLibrary.BreakVector2D` _returnvalue_8) (`.Y` (`KismetMathLibrary.BreakVector2D` _returnvalue_8))) (`KismetMathLibrary.ComposeRotators` _outorientation (struct :`Yaw` -90.0))) (`self.JetpackHorizontalForce`))))
          (`CharacterMovementComponent.AddForce` (`self.CharacterMovement`) (`KismetMathLibrary.MakeVector` _returnvalue_x _returnvalue_y _jetpackverticalforce))
          (else
            (`CharacterMovementComponent.AddForce` (`self.CharacterMovement`) (`KismetMathLibrary.MakeVector` 0.0 0.0 _jetpackverticalforce))))))
    (:`then_4`
      ;[1 1 1] Clamp Velocity for better Jetpack handling
      (if (> (`KismetMathLibrary.VSize` _returnvalue) (`self.MaxVelocity`))
        (`PrimitiveComponent.SetPhysicsLinearVelocity` (`self.CapsuleComponent`) (`KismetMathLibrary.ClampVectorSize` _returnvalue 0.0 (`self.MaxVelocity`)) false "None")))))

(fn `UserConstructionScript`)