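; NewPlanet_BP is a planet actor for a run-on-sphere game that positions itself beneath the player pawn when play begins.
; It moves to the pawn's location, lowered on Z by its Sphere's world Y scale times BaseMultiplierValue from RunOnSphereGameMode.
; The placement runs once without sweep and only if the game mode cast succeeds; Tick, overlap and construction script are empty.
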(event `self.ReceiveBeginPlay`
  (bind (_returnvalue_x _returnvalue_y) (`KismetMathLibrary.BreakVector` (`SceneComponent.K2_GetComponentScale` (`self.Sphere`))))
  (`|ExecutionSequence`
    (:`then_0`
      ;[1 1 1] Set Sphere below Pawn
      (bind _asrun_on_sphere_game_mode (cast `/Game/RunOnSphereGameMode` (`GameplayStatics.GetGameMode`)))
      (`self.K2_SetActorLocation` (+ (- (`self.K2_GetActorLocation` (`GameplayStatics.GetPlayerPawn` 0)) (`KismetMathLibrary.MakeVector` 0.0 0.0 (* _returnvalue_y (`/Game/RunOnSphereGameMode.BaseMultiplierValue` _asrun_on_sphere_game_mode)))) (0.0 0.0 0.0))))))

(event `self.ReceiveTick`
  (params (DeltaSeconds :type "Float (single-precision)")))

(fn `UserConstructionScript`)