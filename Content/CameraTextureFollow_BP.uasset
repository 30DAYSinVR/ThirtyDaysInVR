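; WaveVR actor that shows the headset camera feed on a cube as a picture-in-picture panel.
; BeginPlay checks camera permission after a short delay, requests it if missing, then binds the WaveVR camera texture to the cube's dynamic material and prints its format.
; Tick updates the camera, pins the actor at an offset from whichever supported WaveVR pawn's VR camera, and toggles visibility via right-controller DPad Right.
; EndPlay shuts the camera down.
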(event `self.ReceiveBeginPlay`
  (bind _wavevrcameratexture (`self.WaveVRCameraTexture`))
  (`KismetSystemLibrary.Delay` 3.0)
  (set `self.IsSeeThroughEnabled` true)
  (bind _returnvalue (`WaveVRPermissionManager.isPermissionGranted` "android.permission.CAMERA"))
  (if (not _returnvalue)
    (`KismetSystemLibrary.PrintString` "WVR_CAMERA Permission isn't granted" true true (struct :`R` 1.0 :`G` 0.007289 :`A` 1.0) 10.0)
    (`AndroidPermissionFunctionLibrary.AcquirePermissions` (`self.permission`)))
  (bind _returnvalue_2 (`WaveVRCameraTexture.getCameraTexture` (`self.WaveVRCameraTexture`)))
  (bind _output_get (set `self.CameraTex` _returnvalue_2))
  (`MaterialInstanceDynamic.SetTextureParameterValue` (`self.DynamicCube`) "Tex" _output_get)
  (bind _returnvalue_3 (`WaveVRCameraTexture.getCameraImageFormat` _wavevrcameratexture))
  (bind _returnvalue_4 (`WaveVRCameraTexture.getCameraImageType` _wavevrcameratexture))
  (bind _returnvalue_5 (`WaveVRCameraTexture.getCameraImageWidth` _wavevrcameratexture))
  (bind _returnvalue_6 (`WaveVRCameraTexture.getCameraImageHeight` _wavevrcameratexture))
  (`KismetSystemLibrary.PrintString` (`KismetStringLibrary.Concat_StrStr` (`|GetEnumeratorNameAsString` _returnvalue_3) " : " (`|GetEnumeratorNameAsString` _returnvalue_4) " :" (`KismetStringLibrary.Conv_IntToString` _returnvalue_5) " : " (`KismetStringLibrary.Conv_IntToString` _returnvalue_6))))

(event `self.ReceiveTick`
  (params (DeltaSeconds :type "Float (single-precision)"))
  (`|ExecutionSequence`
    (:`then_0`
      (if (`self.IsSeeThroughEnabled`)
        _
        (else
          _))
      (`WaveVRCameraTexture.updateCamera` (`self.WaveVRCameraTexture`) DeltaSeconds))
    (:`then_1`
      (`self.Update PiP Position`))
    (:`then_2`
      ;[1 1 1] Drafty PiP Control
      (bind _returnvalue (`WaveVRController.IsRightControllerButtonPressed` "DPad_Right"))
      (if _returnvalue
        (bind _output_get (set `self.IsSeeThroughEnabled` (not (`self.IsSeeThroughEnabled`))))
        (`self.SetActorHiddenInGame` _output_get)))))

(event `self.ReceiveEndPlay`
  (params (EndPlayReason :type "EEndPlayReason Enum" :default "Destroyed"))
  (`WaveVRCameraTexture.shutdownCamera` (`self.WaveVRCameraTexture`)))

(fn `Update PiP Position`
  (bind _returnvalue (`GameplayStatics.GetPlayerPawn` 0))
  (bind _pawntargetcamera (`self.PawnTargetCamera`))
  (bind (_returnvalue_location _returnvalue_rotation) (`KismetMathLibrary.BreakTransform` (`SceneComponent.K2_GetComponentToWorld` _pawntargetcamera)))
  (bind _aswave_vr_pawn (cast `/WaveVR/Blueprints/WaveVR_Pawn` _returnvalue)
    (:`then`
      (set `self.PawnTargetCamera` (`/WaveVR/Blueprints/WaveVR_Pawn.VRCamera` _aswave_vr_pawn)))
    (:`CastFailed`
      (bind _asrun_in_place_wave_vr_pawn (cast `/WaveVR/Blueprints/RunInPlace_WaveVR_Pawn` _returnvalue)
        (:`then`
          (set `self.PawnTargetCamera` (`/WaveVR/Blueprints/RunInPlace_WaveVR_Pawn.VRCamera` _asrun_in_place_wave_vr_pawn)))
        (:`CastFailed`
          (bind _asrun_on_sphere_wave_vr_pawn (cast `/WaveVR/Blueprints/RunOnSphere_WaveVR_Pawn` _returnvalue)
            (:`then`
              (set `self.PawnTargetCamera` (`/WaveVR/Blueprints/RunOnSphere_WaveVR_Pawn.VRCamera` _asrun_on_sphere_wave_vr_pawn)))
            (:`CastFailed`
              (bind _asplanet_walker_wave_vr_pawn_bp (cast `/Game/PlanetWalker_WaveVR_Pawn_BP` _returnvalue))
              (set `self.PawnTargetCamera` (`/Game/PlanetWalker_WaveVR_Pawn_BP.VRCamera` _asplanet_walker_wave_vr_pawn_bp))))))))
  (`self.K2_SetActorTransform` (`KismetMathLibrary.MakeTransform` (+ _returnvalue_location (* (`SceneComponent.GetForwardVector` _pawntargetcamera) 300.0) (* (`SceneComponent.GetUpVector` _pawntargetcamera) -100.0) (* (`SceneComponent.GetRightVector` _pawntargetcamera) 50.0)) _returnvalue_rotation)))

(fn `UserConstructionScript`
  (bind _returnvalue (`PrimitiveComponent.CreateDynamicMaterialInstance` (`self.Cube`) 0 null))
  (set `self.DynamicCube` _returnvalue)
  (`KismetSystemLibrary.PrintString` "Camera constructor")
  (`SceneComponent.SetHiddenInGame` (`self.DefaultSceneRoot1`) (`self.IsSeeThroughEnabled`) true))