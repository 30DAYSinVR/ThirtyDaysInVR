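; Planet actor that positions itself beneath the player pawn and scatters collectables around itself at game start.
; On BeginPlay it offsets its center from the pawn using the Sphere's scaled radius plus a fixed vertical shift.
; Three staggered delays share one spawn path, recomputing that center from the pawn's current location and adding a random radius-length vector.
; Each CollectableBP is attached to the planet with KeepRelative rules, with debug prints of locations.
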(event `self.ReceiveBeginPlay`
  (bind (_returnvalue_x _returnvalue_y) (`KismetMathLibrary.BreakVector` (`SceneComponent.K2_GetComponentScale` (`self.Sphere`))))
  (bind (_returnvalue_x_2 _returnvalue_y_2) (`KismetMathLibrary.BreakVector` (`SceneComponent.K2_GetComponentScale` (`self.Sphere`))))
  (bind _returnvalue (+ (- (`self.K2_GetActorLocation` (`GameplayStatics.GetPlayerPawn` 0)) (`KismetMathLibrary.MakeVector` 0.0 0.0 (* _returnvalue_y 100.0))) (0.0 0.0 1000.0)))
  (`|ExecutionSequence`
    (:`then_0`
      ;[1 1 1] Set Sphere below Pawn
      (`self.K2_SetActorLocation` _returnvalue))
    (:`then_1`
      (`KismetSystemLibrary.Delay` 1.0)
      (bind _returnvalue_2 (`|SpawnActorFromClass` (`self.CollectableBP`) (`KismetMathLibrary.MakeTransform` (+ _returnvalue (* (`KismetMathLibrary.RandomUnitVector`) (* _returnvalue_y_2 100.0)))) "AlwaysSpawn" "OverrideRootScale" null null :!label _label))
      (`KismetSystemLibrary.PrintString` (`KismetStringLibrary.Conv_VectorToString` (`self.K2_GetActorLocation` _returnvalue_2)) true true (struct :`R` 1.0 :`B` 0.021336 :`A` 1.0) 10.0)
      (`self.K2_AttachToActor` _returnvalue_2 self "None" "KeepRelative" "KeepRelative" "KeepRelative" false))
    (:`then_2`
      (`KismetSystemLibrary.Delay` 3.0)
      (goto _label))
    (:`then_3`
      (`KismetSystemLibrary.Delay` 5.0)
      (goto _label))
    (:`then_4`
      (`KismetSystemLibrary.PrintString` (`KismetStringLibrary.Conv_VectorToString` (`SceneComponent.K2_GetComponentLocation` (`self.Sphere`)))))))

(event `self.ReceiveTick`
  (params (DeltaSeconds :type "Float (single-precision)")))

(fn `UserConstructionScript`)